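; BP_Door_01 is a door that swings as a grabbed handle is moved.
; Grab and drop events from GrabComponent toggle an IsGrabbed flag checked every Tick.
; While grabbed, the door mesh yaws to face the Sphere with a 90 degree offset; otherwise the Sphere snaps back to the knob.
; A yaw clamp node exists but is unconnected, so the swing is unlimited.
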(event OnGrabbed(GrabComponent)
  (Variables|Default|Setis%20Grabbed true))

(event OnDropped(GrabComponent)
  (Variables|Default|Setis%20Grabbed false))

(event EventTick
  (params (DeltaSeconds :type Float%20%28single-precision%29))
  (bind _mesh_door_02 (Variables|Default|GetMesh_Door_02))
  (if (Variables|Default|Getis%20Grabbed)
    (Transformation|SetWorldRotation _mesh_door_02 (Math|Rotator|MakeRotator 0.0 0.0 (+ (.yaw (Math|Rotator|FindLookatRotation (Transformation|GetWorldLocation _mesh_door_02) (Transformation|GetWorldLocation (Variables|Default|GetSphere)))) 9e+01)) false false)
    (else
      (Transformation|SetWorldLocation (Variables|Default|GetSphere) (Transformation|GetWorldLocation (Variables|Default|GetMesh_Door_Knob_01)) false false))))

(fn ConstructionScript)